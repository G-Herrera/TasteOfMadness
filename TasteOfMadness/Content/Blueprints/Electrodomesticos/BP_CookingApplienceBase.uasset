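; Base cooking appliance that turns its stored ingredients into a finished dish.
; Its Box overlap sets or clears itself as the overlapping appliance on BP_ClareCharacter.
; CocinarPlatillo applies the appliance's output texture to each ingredient, spawns a BP_PlatilloTerminado at the appliance's transform and initializes it with both.
; It then empties the ingredient list and flags itself ready; nothing here fills that list or triggers cooking.
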(event `self.Box.OnComponentBeginOverlap`
  (params (OverlappedComponent :type "PrimitiveComponent Object Reference") (OtherActor :type "Actor Object Reference") (OtherComp :type "PrimitiveComponent Object Reference") (OtherBodyIndex :type Integer) (bFromSweep :type Boolean) (SweepResult :type "HitResult Structure (by ref)"))
  (bind _asbp_clare_character (cast `/Game/Characters/Clare/Blueprints/BP_ClareCharacter` OtherActor))
  (set `/Game/Characters/Clare/Blueprints/BP_ClareCharacter.OverlappingAppliance` self _asbp_clare_character))

(event `self.Box.OnComponentEndOverlap`
  (params (OverlappedComponent :type "PrimitiveComponent Object Reference") (OtherActor :type "Actor Object Reference") (OtherComp :type "PrimitiveComponent Object Reference") (OtherBodyIndex :type Integer))
  (bind _asbp_clare_character (cast `/Game/Characters/Clare/Blueprints/BP_ClareCharacter` OtherActor))
  (set `/Game/Characters/Clare/Blueprints/BP_ClareCharacter.OverlappingAppliance` null _asbp_clare_character))

(fn `CocinarPlatillo`
  (for _array_element (`self.IngredientsArray`)
    (bind _output_get (set `/Game/Blueprints/Ingredientes/BP_IngredientesBase.CurrentTexture` (`self.OutputTexture`) _array_element))
    (`KismetSystemLibrary.PrintString` (`KismetStringLibrary.Concat_StrStr` "Cambiando textura de ingrediente a :  " (`|GetEnumeratorNameAsString` _output_get))))
  (bind _returnvalue (`|SpawnActorFromClass` "/Game/Blueprints/Ingredientes/BP_PlatilloTerminado.BP_PlatilloTerminado_C" (`self.GetTransform`) "Undefined" "OverrideRootScale" null null))
  (bind _output_get_2 (set `self.SpawnedDish` _returnvalue))
  (`/Game/Blueprints/Ingredientes/BP_PlatilloTerminado.InitializeDish` _output_get_2 (`self.IngredientsArray`) (`self.OutputTexture`))
  (`KismetArrayLibrary.Array_Clear` (`self.IngredientsArray`))
  (set `self.IsReady` true)
  (`KismetSystemLibrary.PrintString` "Platillo cocinado y listo"))

(fn `UserConstructionScript`)