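; BP_CajaDeIngredientes is an ingredient crate that spawns random ingredient actors while Clare is nearby.
; Its InteractBox overlap events track a BP_ClareCharacter reference and a nearby flag.
; SpawnIngredient checks that flag, picks a random class from IngredienteClasses and spawns it at a random positive X/Y offset from the crate, storing it as LastSpawnedIngredient.
; Nothing in this Blueprint calls SpawnIngredient, and an empty class list only prints a warning.
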(event `self.InteractBox.OnComponentBeginOverlap`
  (params (OverlappedComponent :type "PrimitiveComponent Object Reference") (OtherActor :type "Actor Object Reference") (OtherComp :type "PrimitiveComponent Object Reference") (OtherBodyIndex :type Integer) (bFromSweep :type Boolean) (SweepResult :type "HitResult Structure (by ref)"))
  (bind _asbp_clare_character (cast `/Game/Characters/Clare/Blueprints/BP_ClareCharacter` OtherActor))
  (set `self.BPClareReference` _asbp_clare_character)
  (set `self.ClareNearby` true))

(event `self.InteractBox.OnComponentEndOverlap`
  (params (OverlappedComponent :type "PrimitiveComponent Object Reference") (OtherActor :type "Actor Object Reference") (OtherComp :type "PrimitiveComponent Object Reference") (OtherBodyIndex :type Integer))
  (cast `/Game/Characters/Clare/Blueprints/BP_ClareCharacter` OtherActor)
  (set `self.ClareNearby` false)
  (set `self.BPClareReference` null))

(fn `SpawnIngredient`
  (if (`self.ClareNearby`)
    (bind _output_get (set `self.ArrayLenght` (`KismetArrayLibrary.Array_Length` (`self.IngredienteClasses`))))
    (if (> _output_get 0)
      (bind _output_get_2 (set `self.RandomIndex` (`KismetMathLibrary.RandomIntegerInRange` 0 (- (`self.ArrayLenght`) 1))))
      (bind _output_get_3 (set `self.SpawnLocation` (+ (`self.K2_GetActorLocation`) (`KismetMathLibrary.MakeVector` (`KismetMathLibrary.Conv_IntToDouble` (`KismetMathLibrary.RandomIntegerInRange` 100 300)) (`KismetMathLibrary.Conv_IntToDouble` (`KismetMathLibrary.RandomIntegerInRange` 100 300))))))
      (bind _returnvalue (`|SpawnActorFromClass` (`|GetArrayItem` (`self.IngredienteClasses`) _output_get_2) (`KismetMathLibrary.MakeTransform` _output_get_3) "AdjustIfPossibleButAlwaysSpawn" "OverrideRootScale" null null))
      (set `self.LastSpawnedIngredient` _returnvalue)
      (return)
      (else
        (`KismetSystemLibrary.PrintString` "SpawnINGREDIENT: IngredienteClasses vacío")))
    (else
      (return))))

(fn `UserConstructionScript`)