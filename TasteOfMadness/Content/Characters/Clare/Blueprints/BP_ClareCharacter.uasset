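; Player character Clare for a cooking game with combat: she gathers ingredients, cooks at appliances, takes orders from Francis and attacks with a knife.
; A timer-driven hand-socket sphere hits swarm enemies or damages Francis once per swing, raising madness; its delayed-enable event is empty.
; BeginPlay spawns hidden tools on the hand socket for SelectToolByIndex to switch.
; An interaction capsule tracks nearby Francis; toolbar creation is unfinished.
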(event `KnifePrimaryAttack`
  ;[1 1 1] Logica ataque con cuchillo
  (if (!= (`self.IsPerformingAttack`) true)
    (set `self.IsPerformingAttack` true)
    (set `self.HasHitThisAttack` false)
    (`self.PlayAnimMontage` (`self.KnifeAttackMontage`))
    (`KismetSystemLibrary.K2_SetTimerDelegate` (delegate `EnableAttackCollision`) (`self.AttackEnableDelay`))
    (`PrimitiveComponent.SetCollisionEnabled` (`self.AttackSphere`) "QueryOnly")
    (set `PrimitiveComponent.bGenerateOverlapEvents` true (`self.AttackSphere`))
    (`KismetSystemLibrary.K2_SetTimerDelegate` (delegate `DisableAttackCollision`) (`self.AttackEnableDuration`))))

(event `DisableAttackCollision`
  ;[1 1 1] Logica ataque con cuchillo
  (`PrimitiveComponent.SetCollisionEnabled` (`self.AttackSphere`) "NoCollision")
  (`KismetSystemLibrary.K2_SetTimerDelegate` (delegate `ResetAttackState`) (`self.AttackResetDelay`)))

(event `EnableAttackCollision`
  ;[1 1 1] Logica ataque con cuchillo
)

(event `ResetAttackState`
  ;[1 1 1] Logica ataque con cuchillo
  (set `self.IsPerformingAttack` false)
  (set `self.HasHitThisAttack` false))

(event `self.AttackSphere.OnComponentBeginOverlap`
  (params (OverlappedComponent :type "PrimitiveComponent Object Reference") (OtherActor :type "Actor Object Reference") (OtherComp :type "PrimitiveComponent Object Reference") (OtherBodyIndex :type Integer) (bFromSweep :type Boolean) (SweepResult :type "HitResult Structure (by ref)"))
  ;[1 1 1] Logica ataque con cuchillo
  (bind _asbp_swarm_enemy (cast `/Game/Characters/Enemies/BP_Rata/BP_SwarmEnemy` OtherActor)
    (:`then`
      (if (`self.IsPerformingAttack`)
        (`KismetSystemLibrary.PrintString` "\"Golpe aplicado\"")
        (`/Game/Characters/Enemies/BP_Rata/BP_SwarmEnemy.RecibirDaño` _asbp_swarm_enemy)))
    (:`CastFailed`
      (bind _asbp_francis_ia (cast `/Game/Characters/Francis/Blueprints/BP_FrancisIA` OtherActor))
      (set `self.As BP Francis IA` _asbp_francis_ia)
      (if (== (`self.HasHitThisAttack`) false)
        (set `self.HasHitThisAttack` true)
        (`GameplayStatics.ApplyDamage` (`self.As BP Francis IA`) (`self.AttackDamage`) (`self.GetController`) self)
        (`/Game/Characters/Clare/Components/BP_MadnessComponent.ChangeMadness` (`self.BP_MadnessComponent`) 10.0)
        (`KismetSystemLibrary.PrintString` "Se resto vida a Francis")))))

(event `PickIngredient`
  ;[1 1 1] Logica para recoger ingredientes
  (if (not (== (`self.OverlappingIngredient`) null))
    (`KismetArrayLibrary.Array_Add` (`self.IngredientsInventory`) (`self.OverlappingIngredient`))
    (`self.K2_DestroyActor` (`self.OverlappingIngredient`))
    (set `self.OverlappingIngredient` null)))

(event `TryCook`
  ;[1 1 1] Logica para cocinar (Remueve del inventario los ingredientes y lo manda a cocinar)
  (if (> (`KismetArrayLibrary.Array_Length` (`self.IngredientsInventory`)) 1)
    (`/Game/Blueprints/Electrodomesticos/BP_CookingApplienceBase.CocinarPlatillo` (`self.OverlappingAppliance`))
    (`KismetArrayLibrary.Array_Remove` (`self.IngredientsInventory`))
    (`KismetSystemLibrary.PrintString` "Clare Esta cocinando" true true (struct :`R` 0.057249 :`G` 1.0 :`A` 1.0) 3.0)
    (else
      (`KismetSystemLibrary.PrintString` "No hay ingredientes para cocinar"))))

(event `ClareDie`
  ;[1 1 1] Evento que llama a la muerte de Clare (desactiva controles)
  (set `self.IsDead` true)
  (`self.DisableInput` (`GameplayStatics.GetPlayerController` 0))
  (`CharacterMovementComponent.DisableMovement` (`self.CharacterMovement`))
  (`KismetSystemLibrary.PrintString` "CLARE A MUERTO" true true (struct :`R` 1.0 :`G` 0.039766 :`A` 1.0) 5.0))

(event `self.ReceiveBeginPlay`
  (bind _attacksphere (`self.AttackSphere`))
  ;[1 1 1] Assignación de herramienta a Clare desde el BeginPlay
  (`SceneComponent.K2_AttachToComponent` (`self.AttackSphere`) (`self.Mesh`) "hand_rSocket" "SnapToTarget" "SnapToTarget" "KeepRelative" true)
  (`SphereComponent.SetSphereRadius` (`self.AttackSphere`) (`self.AttackSphereRadius`) true)
  (`PrimitiveComponent.SetCollisionEnabled` _attacksphere "NoCollision")
  (set `PrimitiveComponent.bGenerateOverlapEvents` true _attacksphere)
  (for _array_element (`self.ToolsActorsArray`)
    (bind _returnvalue (`|SpawnActorFromClass` _array_element (`KismetMathLibrary.MakeTransform` (0.0 0.0 0.0)) "Undefined" "OverrideRootScale" null null))
    (`self.K2_AttachToComponent` _returnvalue (`self.Mesh`) "hand_rSocket" "SnapToTarget" "SnapToTarget" "KeepWorld" true)
    (`KismetArrayLibrary.Array_Add` (`self.SpawnedToolsArray`) _returnvalue)
    (`self.SetActorHiddenInGame` _returnvalue true)
    (`KismetSystemLibrary.PrintString` (`KismetSystemLibrary.GetDisplayName` _returnvalue))
    (`self.CreateToolBar`)))

(event `CreateToolBar`
  ;[1 1 1] Asignación de herramientas a HUD (SIN FUNCIONAR AUN)
)

(event `self.InteractionCapsule.OnComponentBeginOverlap`
  (params (OverlappedComponent :type "PrimitiveComponent Object Reference") (OtherActor :type "Actor Object Reference") (OtherComp :type "PrimitiveComponent Object Reference") (OtherBodyIndex :type Integer) (bFromSweep :type Boolean) (SweepResult :type "HitResult Structure (by ref)"))
  ;[1 1 1] Logica detección de Francis para tomar pedido
  (bind _asbp_francis_ia (cast `/Game/Characters/Francis/Blueprints/BP_FrancisIA` OtherActor))
  (set `self.NearbyFrancis` _asbp_francis_ia))

(event `self.InteractionCapsule.OnComponentEndOverlap`
  (params (OverlappedComponent :type "PrimitiveComponent Object Reference") (OtherActor :type "Actor Object Reference") (OtherComp :type "PrimitiveComponent Object Reference") (OtherBodyIndex :type Integer))
  ;[1 1 1] Logica detección de Francis para tomar pedido
  (bind _asbp_francis_ia (cast `/Game/Characters/Francis/Blueprints/BP_FrancisIA` OtherActor))
  (if (== _asbp_francis_ia (`self.NearbyFrancis`))
    (set `self.NearbyFrancis` null)))

(fn `CollectOrder`
  (params (Francis :type "/Game/Characters/Francis/Blueprints/BP_FrancisIA Object Reference"))
  (bind _nearbyfrancis (`self.NearbyFrancis`))
  (`KismetArrayLibrary.Array_Add` (`self.CollectedOrders`) (`/Game/Characters/Francis/Blueprints/BP_FrancisIA.OrderData` Francis))
  (set `/Game/Characters/Francis/Blueprints/BP_FrancisIA.HasOrder` false _nearbyfrancis)
  (set `/Game/Characters/Francis/Blueprints/BP_FrancisIA.OrderData` (make `/Game/Characters/Francis/Components/S_OrderData` null) _nearbyfrancis))

(fn `SelectToolByIndex`
  (params (Index :type Integer))
  (locals (IndexLocal :type Integer))
  (bind _output (`|GetArrayItem` (`self.SpawnedToolsArray`) (`local.IndexLocal`)))
  (set `local.IndexLocal` Index)
  (if (and (>= (`local.IndexLocal`) 0) (< (`local.IndexLocal`) (`KismetArrayLibrary.Array_Length` (`self.ToolsArray`))))
    (set `self.CurrentTools` (`|GetArrayItem` (`self.ToolsArray`) (`local.IndexLocal`)))
    (for _array_element (`self.SpawnedToolsArray`)
      (`self.SetActorHiddenInGame` _array_element true)
      (`self.SetActorEnableCollision` _array_element false))
    (`/Engine/EditorBlueprintResources/StandardMacros.IsValid` _output
      (:`Is Valid`
        (bind _output_get (set `self.CurrentToolActor` _output))
        (`self.SetActorHiddenInGame` _output_get false)
        (`self.SetActorEnableCollision` _output_get true)
        (`self.K2_AttachToComponent` (`self.CurrentToolActor`) (`self.Mesh`) "hand_rSocket" "SnapToTarget" "SnapToTarget" "SnapToTarget" false)
        (return)))
    (else
      (`KismetSystemLibrary.PrintString` (`KismetStringLibrary.Concat_StrStr` "Index fuera de rango" (`KismetStringLibrary.Conv_IntToString` (`local.IndexLocal`)))))))

(fn `UserConstructionScript`)