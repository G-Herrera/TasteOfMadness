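; Player controller for Clare in a cooking game with knife combat, handling HUD, menus and input.
; It binds health and madness component events to the HUD, toggles the collected-orders notepad widget and opens the pause menu.
; Input drives world-axis movement, tool selection, order taking and a prioritized interact chain: knife, cook, ingredient box, plate pickup, delivery to Francis, ingredient pickup.
; Tool selection relies on a character reference cached only by the interact key.
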(event `self.ReceiveBeginPlay`
  (`self.SetupHUD`))

(event `SetupHUD`
  ;[1 1 1] Setting HUD
  (bind _returnvalue (`|CreateWidget` "/Game/Characters/Clare/Widgets/WBP_ClareHealth.WBP_ClareHealth_C" (`GameplayStatics.GetPlayerController` 0)))
  (set `self.HealthHUD` _returnvalue)
  (`UserWidget.AddToViewport` _returnvalue 0)
  (bind _asbp_clare_character (cast `/Game/Characters/Clare/Blueprints/BP_ClareCharacter` (`self.K2_GetPawn`)))
  (add `/Game/Characters/Clare/Components/BP_HealthComponent.OnHealthChanged` (`/Game/Characters/Clare/Blueprints/BP_ClareCharacter.BP_HealthComponent` _asbp_clare_character) (delegate `SetHealth`))
  (bind _asbp_clare_character_2 (cast `/Game/Characters/Clare/Blueprints/BP_ClareCharacter` (`self.K2_GetPawn`)))
  (add `/Game/Characters/Clare/Components/BP_MadnessComponent.OnMadnessChanged` (`/Game/Characters/Clare/Blueprints/BP_ClareCharacter.BP_MadnessComponent` _asbp_clare_character_2) (delegate `SetMadness`)))

(event `InputAction|AbrirComandas`
  (params (Key :type "Key Structure"))
  (bind _comandawidget (`self.ComandaWidget`))
  ;[1 1 1] Logica para abrir, cerrar y actualizar libreta de comandas
  (:`Pressed`
    (if (`self.IsComandaVisible`)
      (`self.ComandaWidget`
        (:`then`
          (`Widget.RemoveFromParent` (`self.ComandaWidget`))
          (set `self.bShowMouseCursor` false)
          (set `self.IsComandaVisible` false)
          (`KismetSystemLibrary.PrintString` "ComandaWidget cerrada" true true (struct :`R` 1.0 :`B` 0.755718 :`A` 1.0) 5.0))
        (:`else`
          (`KismetSystemLibrary.PrintString` "ComandaWidget inválido al intentar cerrar" true true (struct :`R` 1.0 :`B` 0.755718 :`A` 1.0) 5.0)))
      (else
        (`self.ComandaWidget`
          (:`then`
            (set `self.bShowMouseCursor` true)
            (`UserWidget.AddToViewport` _comandawidget 0)
            (bind _asbp_clare_character (cast `/Game/Characters/Clare/Blueprints/BP_ClareCharacter` (`self.K2_GetPawn`)))
            (`/Game/Characters/Clare/Widgets/WBP_ComandaOrdenes.RefresList` _comandawidget (`/Game/Characters/Clare/Blueprints/BP_ClareCharacter.CollectedOrders` _asbp_clare_character))
            (set `self.IsComandaVisible` true))
          (:`else`
            (bind _returnvalue (`|CreateWidget` "/Game/Characters/Clare/Widgets/WBP_ComandaOrdenes.WBP_ComandaOrdenes_C" self))
            (bind _output_get (set `self.ComandaWidget` _returnvalue))
            (set `self.bShowMouseCursor` false)
            (`UserWidget.AddToViewport` _output_get 0)
            (bind _asbp_clare_character_2 (cast `/Game/Characters/Clare/Blueprints/BP_ClareCharacter` (`self.K2_GetPawn`)))
            (`/Game/Characters/Clare/Widgets/WBP_ComandaOrdenes.RefresList` _output_get (`/Game/Characters/Clare/Blueprints/BP_ClareCharacter.CollectedOrders` _asbp_clare_character_2))
            (set `self.IsComandaVisible` true)
            (`KismetSystemLibrary.PrintString` "ComandaWidget creada" true true (struct :`R` 1.0 :`B` 0.755718 :`A` 1.0) 5.0)))))))

(event `SetHealth`
  (params (CurrentHealth :type "Float (double-precision)") (MaxHealth :type "Float (double-precision)"))
  ;[1 1 1] Setting HUD
  (`/Game/Characters/Clare/Widgets/WBP_ClareHealth.SetHealth` (`self.HealthHUD`) CurrentHealth MaxHealth))

(event `SetMadness`
  (params (CurrentMadness :type "Float (double-precision)") (MaxMadness :type "Float (double-precision)"))
  ;[1 1 1] Setting HUD
  (`/Game/Characters/Clare/Widgets/WBP_ClareHealth.SetMadness` (`self.HealthHUD`) CurrentMadness MaxMadness))

(event `InputAxis|MoveForward`
  (params (AxisValue :type "Float (single-precision)"))
  (bind _returnvalue (`self.K2_GetPawn`))
  ;[1 1 1] Moviemiento arriba y abajo
  (`/Engine/EditorBlueprintResources/StandardMacros.IsValid` _returnvalue
    (:`Is Valid`
      (`Pawn.AddMovementInput` _returnvalue (-1.0 0.0 0.0) AxisValue false))))

(event `InputAxis|MoveRight`
  (params (AxisValue :type "Float (single-precision)"))
  (bind _returnvalue (`self.K2_GetPawn`))
  ;[1 1 1] Moviento lados
  (`/Engine/EditorBlueprintResources/StandardMacros.IsValid` _returnvalue
    (:`Is Valid`
      (`Pawn.AddMovementInput` _returnvalue (0.0 -1.0 0.0) AxisValue false))))

(event `InputAction|TakeOrder`
  (params (Key :type "Key Structure"))
  ;[1 1 1] Input para recoger pedido
  (:`Pressed`
    (bind _asbp_clare_character (cast `/Game/Characters/Clare/Blueprints/BP_ClareCharacter` (`self.K2_GetPawn`))
      (:`then`
        (bind _output_get (set `self.Nearby Francis` (`/Game/Characters/Clare/Blueprints/BP_ClareCharacter.NearbyFrancis` _asbp_clare_character)))
        (`/Engine/EditorBlueprintResources/StandardMacros.IsValid` _output_get
          (:`Is Valid`
            (`KismetSystemLibrary.PrintString` (`KismetStringLibrary.Concat_StrStr` "TakeOrder: NearbyFrancis = " (`KismetSystemLibrary.GetDisplayName` _output_get)))
            (bind _asbp_francis_ia (cast `/Game/Characters/Francis/Blueprints/BP_FrancisIA` (`self.Nearby Francis`)))
            (if (`/Game/Characters/Francis/Blueprints/BP_FrancisIA.HasOrder` _asbp_francis_ia)
              (`/Game/Characters/Clare/Blueprints/BP_ClareCharacter.CollectOrder` (`self.As BP Clare Character`) (`self.Nearby Francis`))
              (`KismetSystemLibrary.PrintString` "TakeOrder: CollectOrder llamado OK")
              (else
                (`KismetSystemLibrary.PrintString` "TakeOrder: NearbyFrancis no tiene pedido (HasOrder = false)"))))
          (:`Is Not Valid`
            (`KismetSystemLibrary.PrintString` "TakeOrder: NearbyFrancis = NONE" true true (struct :`R` 0.991265 :`B` 1.0 :`A` 1.0) 5.0))))
      (:`CastFailed`
        (`KismetSystemLibrary.PrintString` "TakeOrder: Controlle pawn no es Clare (Cast failed)" true true (struct :`R` 0.991265 :`B` 1.0 :`A` 1.0) 5.0)))))

(event `InputAction|Tool1`
  (params (Key :type "Key Structure"))
  ;[1 1 1] Input de Seleccion de herramienta
  (:`Pressed`
    (bind _asbp_clare_character (cast `/Game/Characters/Clare/Blueprints/BP_ClareCharacter` (`self.As BP Clare Character`)))
    (`/Game/Characters/Clare/Blueprints/BP_ClareCharacter.SelectToolByIndex` _asbp_clare_character 6)))

(event `InputAction|Tool5`
  (params (Key :type "Key Structure"))
  ;[1 1 1] Input de Seleccion de herramienta
)

(event `InputAction|Tool6`
  (params (Key :type "Key Structure"))
  ;[1 1 1] Input de Seleccion de herramienta
)

(event `InputAction|Tool2`
  (params (Key :type "Key Structure"))
  ;[1 1 1] Input de Seleccion de herramienta
  (:`Pressed`
    (bind _asbp_clare_character (cast `/Game/Characters/Clare/Blueprints/BP_ClareCharacter` (`self.As BP Clare Character`)))
    (`/Game/Characters/Clare/Blueprints/BP_ClareCharacter.SelectToolByIndex` _asbp_clare_character 0)))

(event `InputAction|Tool7`
  (params (Key :type "Key Structure"))
  ;[1 1 1] Input de Seleccion de herramienta
)

(event `InputAction|Tool3`
  (params (Key :type "Key Structure"))
  ;[1 1 1] Input de Seleccion de herramienta
  (:`Pressed`
    (bind _asbp_clare_character (cast `/Game/Characters/Clare/Blueprints/BP_ClareCharacter` (`self.As BP Clare Character`)))
    (`/Game/Characters/Clare/Blueprints/BP_ClareCharacter.SelectToolByIndex` _asbp_clare_character 1)))

(event `InputAction|Tool4`
  (params (Key :type "Key Structure"))
  ;[1 1 1] Input de Seleccion de herramienta
)

(event `InputAction|AbrirCaja`
  (params (Key :type "Key Structure"))
  (:`Pressed`
    (bind _asbp_ingredient_box (cast `/Game/System/Orders/Blueprints/BP_IngredientBox` (`self.IngredienteBoxRef`)))
    (`/Game/System/Orders/Blueprints/BP_IngredientBox.AbrirCaja` _asbp_ingredient_box)))

(event `InputAction|InteractionKey`
  (params (Key :type "Key Structure"))
  (bind _as_bp_clare_character (`self.As BP Clare Character`))
  (bind _as_bp_clare_character_2 (`self.As BP Clare Character`))
  (bind _as_bp_clare_character_3 (`self.As BP Clare Character`))
  (bind _as_bp_clare_character_4 (`self.As BP Clare Character`))
  ;[1 1 1] KnifeAttack
  (:`Pressed`
    (bind _asbp_clare_character (cast `/Game/Characters/Clare/Blueprints/BP_ClareCharacter` (`self.K2_GetPawn`)))
    (set `self.As BP Clare Character` _asbp_clare_character)
    (if (and (`|EnumEquality` (`/Game/Characters/Clare/Blueprints/BP_ClareCharacter.CurrentTools` _as_bp_clare_character_4) "NewEnumerator6") (`/Game/Characters/Clare/Blueprints/BP_ClareCharacter.CanAttack` _as_bp_clare_character_4))
      (`/Game/Characters/Clare/Blueprints/BP_ClareCharacter.KnifePrimaryAttack` (`self.As BP Clare Character`))
      (elif (!= (`/Game/Characters/Clare/Blueprints/BP_ClareCharacter.OverlappingAppliance` (`self.As BP Clare Character`)) null)
        (`/Game/Characters/Clare/Blueprints/BP_ClareCharacter.TryCook` (`self.As BP Clare Character`))
        (elif (!= (`/Game/Characters/Clare/Blueprints/BP_ClareCharacter.NearByIngredientBox` (`self.As BP Clare Character`)) null)
          (`/Game/Blueprints/Enviroment/BP_CajaDeIngredientes.SpawnIngredient` (`/Game/Characters/Clare/Blueprints/BP_ClareCharacter.NearByIngredientBox` (`self.As BP Clare Character`)))
          (elif (!= (`/Game/Characters/Clare/Blueprints/BP_ClareCharacter.NearByPlatillo` (`self.As BP Clare Character`)) null)
            (`/Game/Characters/Clare/Blueprints/BP_ClareCharacter.PickUpPlate` _as_bp_clare_character (`/Game/Characters/Clare/Blueprints/BP_ClareCharacter.NearByPlatillo` _as_bp_clare_character))
            (else
              (bind _nearbyfrancis (`/Game/Characters/Clare/Blueprints/BP_ClareCharacter.NearbyFrancis` (`self.As BP Clare Character`))
                (:`then`
                  (set `self.Nearby Francis` _nearbyfrancis)
                  (if (`/Game/Characters/Clare/Blueprints/BP_ClareCharacter.HasHeldPlate` (`self.As BP Clare Character`))
                    (`/Game/Characters/Francis/Blueprints/BP_FrancisIA.RecibirPlatillo` (`self.Nearby Francis`) (`/Game/Characters/Clare/Blueprints/BP_ClareCharacter.HeldPlateTexture` _as_bp_clare_character_2) _as_bp_clare_character_2)
                    (set `/Game/Characters/Clare/Blueprints/BP_ClareCharacter.HasHeldPlate` false _as_bp_clare_character_3)
                    (set `/Game/Characters/Clare/Blueprints/BP_ClareCharacter.HeldPlateTexture` "NewEnumerator7" _as_bp_clare_character_3)
                    (else
                      (`KismetSystemLibrary.PrintString` "No tienes platillo que entregar"))))
                (:`else`
                  (`/Game/Characters/Clare/Blueprints/BP_ClareCharacter.PickIngredient` (`self.As BP Clare Character`)))))))))))

(event `InputAction|PAUSA`
  (params (Key :type "Key Structure"))
  (:`Pressed`
    (`GameplayStatics.SetGamePaused` true)
    (bind _returnvalue (`|CreateWidget` "/Game/UI/Widgets/WBP_PauseMenu.WBP_PauseMenu_C"))
    (`UserWidget.AddToViewport` _returnvalue 0)
    (`WidgetBlueprintLibrary.SetInputMode_UIOnlyEx` null null)
    (set `self.bShowMouseCursor` true)))

(fn `UserConstructionScript`)