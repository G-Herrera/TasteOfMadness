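; BP_GameManager runs the Clare match, spawning Francis actors and deciding victory or defeat.
; After a short delay on BeginPlay, SpawnFrancis spawns behind SpawnPoint and re-arms itself on a random timer until the spawn total is reached.
; Tick compares dead Francis and successful order counts against thresholds, checking defeat first.
; Either outcome prints a message, pauses the game and shows its end-screen widget with UI-only input.
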(event `self.ReceiveBeginPlay`
  (set `self.SpawnCount` 0)
  (`KismetSystemLibrary.Delay` 2.0)
  (`KismetSystemLibrary.K2_SetTimer` self "SpawnFrancis" 0.1))

(event `self.ReceiveTick`
  (params (DeltaSeconds :type "Float (single-precision)"))
  (if (> (`self.FrancisMuertos`) (`self.LoseThreshold`))
    (`self.Defeat`)
    (elif (>= (`self.PedidosExitosos`) (`self.WinThreshold`))
      (`self.Victory`))))

(fn `Defeat`
  (bind _returnvalue (`GameplayStatics.GetPlayerController` 0))
  (`KismetSystemLibrary.PrintString` "CLARE HA PERDIDO" true true (struct :`G` 1.0 :`B` 0.101517 :`A` 1.0) 20.0)
  (`GameplayStatics.SetGamePaused` true)
  (bind _returnvalue_2 (`|CreateWidget` "/Game/UI/Widgets/WBP_GameOver.WBP_GameOver_C"))
  (`UserWidget.AddToViewport` _returnvalue_2 0)
  (set `PlayerController.bShowMouseCursor` true _returnvalue)
  (`WidgetBlueprintLibrary.SetInputMode_UIOnlyEx` _returnvalue _returnvalue_2))

(fn `SpawnFrancis`
  (if (< (`self.SpawnCount`) (`self.TotalFrancistoSpawn`))
    (`|SpawnActorFromClass` (`self.FrancisReference`) (`KismetMathLibrary.MakeTransform` (+ (* (`self.GetActorForwardVector` (`self.SpawnPoint`)) -300.0) (`self.K2_GetActorLocation` (`self.SpawnPoint`)))) "AdjustIfPossibleButAlwaysSpawn" "OverrideRootScale" null null)
    (bind _result (`/Engine/EditorBlueprintResources/StandardMacros.IncrementInt` (`self.SpawnCount`))
      (:`  `
        (set `self.SpawnCount` _result)
        (`KismetSystemLibrary.K2_SetTimer` self "SpawnFrancis" (`KismetMathLibrary.RandomFloatInRange` 5.0 10.0))))
    (else
      (return))))

(fn `UserConstructionScript`)

(fn `Victory`
  (bind _returnvalue (`GameplayStatics.GetPlayerController` 0))
  (`KismetSystemLibrary.PrintString` "CLARE HA GANADO" true true (struct :`G` 1.0 :`B` 0.101517 :`A` 1.0) 20.0)
  (`GameplayStatics.SetGamePaused` true)
  (bind _returnvalue_2 (`|CreateWidget` "/Game/UI/Widgets/WBP_YouWin.WBP_YouWin_C"))
  (`UserWidget.AddToViewport` _returnvalue_2 0)
  (set `PlayerController.bShowMouseCursor` true _returnvalue)
  (`WidgetBlueprintLibrary.SetInputMode_UIOnlyEx` _returnvalue _returnvalue_2))