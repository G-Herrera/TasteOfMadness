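; Health component for Clare that tracks current health and reacts to damage taken by its owning actor.
; On BeginPlay it fills health to the maximum and binds to the owner's any-damage event, guarded by a bound flag.
; Each hit lowers clamped health and broadcasts the change.
; The depletion check recomputes the subtraction on the updated health, so depletion can fire one equal hit before zero.
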(event `self.ReceiveBeginPlay`
  (bind _returnvalue (`self.GetOwner`))
  ;[1 1 1] Logica de vida de Clare
  (set `self.CurrentHealth` (`self.MaxHealth`))
  (`/Engine/EditorBlueprintResources/StandardMacros.IsValid` _returnvalue
    (:`Is Valid`
      (if (`self.bIsBound`)
        (`KismetSystemLibrary.PrintString` "BOUND TO DAMAGE EVENT")
        (else
          (add `Actor.OnTakeAnyDamage` _returnvalue (delegate `OnDamageTaken`))
          (set `self.bIsBound` true))))))

(event `OnDamageTaken`
  (params (DamagedActor :type "Actor Object Reference") (Damage :type "Float (double-precision)") (DamageType :type "DamageType Object Reference") (InstigatedBy :type "Controller Object Reference") (DamageCauser :type "Actor Object Reference"))
  (bind _returnvalue (`KismetMathLibrary.FClamp` (- (`self.CurrentHealth`) Damage) 0.0 (`self.MaxHealth`)))
  ;[1 1 1] Logica de vida de Clare
  (set `self.CurrentHealth` _returnvalue)
  (`self.OnHealthChanged` (`self.CurrentHealth`) (`self.MaxHealth`))
  (if (<= _returnvalue 0.0)
    (`self.OnHealthDepleted`)))