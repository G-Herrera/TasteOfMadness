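; BP_SwarmEnemy is a swarm enemy, filed under the rat enemy assets, that chases the player character and shows a health bar.
; When PawnSensing sees a BP_ClareCharacter, it prints a debug message and issues AIMoveTo toward that character.
; On BeginPlay it registers itself as the owner of its health bar widget.
; Every tick it updates the bar from BarraVidaEnemie and rotates the widget to face the player camera.
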(event `self.ReceiveBeginPlay`
  (bind _aswbp_health_bar (cast `/Game/Characters/Content_Enemies/BP_Rata/WBP_HealthBar` (`WidgetComponent.GetUserWidgetObject` (`self.HealthBarWidget`))))
  (set `/Game/Characters/Content_Enemies/BP_Rata/WBP_HealthBar.OwnerEnemy` self _aswbp_health_bar))

(event `self.PawnSensing.OnSeePawn`
  (params (Pawn :type "Pawn Object Reference"))
  (bind _asbp_clare_character (cast `/Game/Characters/Clare/Blueprints/BP_ClareCharacter` Pawn))
  (`KismetSystemLibrary.PrintString` "\"Përsiguiendo\"")
  (`|AIMoveTo` self (0.0 0.0 0.0) _asbp_clare_character 100.0))

(event `self.ReceiveTick`
  (params (DeltaSeconds :type "Float (single-precision)"))
  (bind _healthbarwidget (`self.HealthBarWidget`))
  (bind _aswbp_health_bar (cast `/Game/Characters/Content_Enemies/BP_Rata/WBP_HealthBar` (`WidgetComponent.GetWidget` (`self.HealthBarWidget`))))
  (`ProgressBar.SetPercent` (`/Game/Characters/Content_Enemies/BP_Rata/WBP_HealthBar.ProgressBar_Health` _aswbp_health_bar) (/ (`self.Barra_VidaEnemie`) 100.0))
  (`SceneComponent.K2_SetWorldRotation` _healthbarwidget (`KismetMathLibrary.FindLookAtRotation` (`SceneComponent.K2_GetComponentLocation` _healthbarwidget) (`SceneComponent.K2_GetComponentLocation` (`PlayerCameraManager.TransformComponent` (`GameplayStatics.GetPlayerCameraManager` 0)))) false false))

(fn `UserConstructionScript`)