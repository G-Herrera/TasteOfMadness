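; Turtle-shell enemy character that spots BP_ClareCharacter through PawnSensing, chases it with AIMoveTo and attacks once on arrival, as StarAttackLoop is an empty stub.
; Attack briefly enables a hitbox that applies damage; Tick drives a camera-facing health bar from BarraVida.
; Event names look swapped: Morir subtracts a separate Health variable and calls itself at zero.
; RecibirDaño, uncalled here, spawns a random ingredient and destroys the actor.
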(event `self.ReceiveTick`
  (params (DeltaSeconds :type "Float (single-precision)"))
  (bind _healthbarwidget (`self.HealthBarWidget`))
  ;[1 1 1] Actualización en Tick: Velocidad, Barra de Vida y Orientación hacia la Cámara
  (`|ExecutionSequence`
    (:`then_0`
      (set `self.Velocidad` (`KismetMathLibrary.VSize` (`self.GetVelocity`))))
    (:`then_1`
      (bind _aswbp_health_bar (cast `/Game/Characters/Enemies/BP_Rata/WBP_HealthBar` (`WidgetComponent.GetWidget` (`self.HealthBarWidget`))))
      (`ProgressBar.SetPercent` (`/Game/Characters/Enemies/BP_Rata/WBP_HealthBar.ProgressBar_Health` _aswbp_health_bar) (/ (`self.BarraVida`) 100.0))
      (`SceneComponent.K2_SetWorldRotation` _healthbarwidget (`KismetMathLibrary.FindLookAtRotation` (`SceneComponent.K2_GetComponentLocation` _healthbarwidget) (`SceneComponent.K2_GetComponentLocation` (`PlayerCameraManager.TransformComponent` (`GameplayStatics.GetPlayerCameraManager` 0)))) false false))))

(event `Attack`
  ;[1 1 1] Ejecución del Ataque (Activar/Desactivar Colisión y Estado de Animación)
  (cast `/Game/Characters/Enemies/Lombriz/ABP_TurtleShell` (`SkeletalMeshComponent.GetAnimInstance` (`self.Mesh`)))
  (set `self.IsAttacking` true)
  (`PrimitiveComponent.SetCollisionEnabled` (`self.AttackHitBox`) "QueryOnly")
  (`KismetSystemLibrary.Delay` 0.5)
  (`PrimitiveComponent.SetCollisionEnabled` (`self.AttackHitBox`) "NoCollision")
  (cast `/Game/Characters/Enemies/Lombriz/ABP_TurtleShell` (`SkeletalMeshComponent.GetAnimInstance` (`self.Mesh`)))
  (set `self.IsAttacking` false))

(event `self.PawnSensing.OnSeePawn`
  (params (Pawn :type "Pawn Object Reference"))
  ;[1 1 1] Detección del Jugador, Persecución y Bucle de Ataque
  (bind _asbp_clare_character (cast `/Game/Characters/Clare/Blueprints/BP_ClareCharacter` Pawn))
  (bind _output_get (set `self.PlayerRef` _asbp_clare_character))
  (set `self.CanAttack` true)
  (`|AIMoveTo` self (0.0 0.0 0.0) _output_get 100.0
    (:`OnSuccess`
      (`self.StarAttackLoop`)
      (`KismetSystemLibrary.Delay` 1.0)
      (if (`self.CanAttack`)
        (`self.Attack`)
        (`self.StarAttackLoop`)))))

(event `StarAttackLoop`
  ;[1 1 1] Detección del Jugador, Persecución y Bucle de Ataque
)

(event `self.AttackHitBox.OnComponentBeginOverlap`
  (params (OverlappedComponent :type "PrimitiveComponent Object Reference") (OtherActor :type "Actor Object Reference") (OtherComp :type "PrimitiveComponent Object Reference") (OtherBodyIndex :type Integer) (bFromSweep :type Boolean) (SweepResult :type "HitResult Structure (by ref)"))
  ;[1 1 1] “Colisión de ataque del enemigo (daño al jugador)”
  (bind _asbp_clare_character (cast `/Game/Characters/Clare/Blueprints/BP_ClareCharacter` OtherActor))
  (if true
    (`GameplayStatics.ApplyDamage` _asbp_clare_character (`self.DañoAtaque`) (`self.GetController`) self)))

(event `Morir`
  ;[1 1 1] Recibir Daño
  (bind _output_get (set `self.Health` (- (`self.Health`) 20.0)))
  (if (<= _output_get 0.0)
    (`self.Morir`)))

(event `RecibirDaño`
  (bind _ingredientesarray (`self.IngredientesArray`))
  ;[1 1 1] Morir
  (`|SpawnActorFromClass` (`|GetArrayItem` _ingredientesarray (`KismetMathLibrary.RandomIntegerInRange` 0 (- (`KismetArrayLibrary.Array_Length` _ingredientesarray) 1))) (`KismetMathLibrary.MakeTransform` (`self.K2_GetActorLocation`) (`self.K2_GetActorRotation`)) "Undefined" "OverrideRootScale" null null)
  (`self.K2_DestroyActor`))

(event `self.AttackRange.OnComponentBeginOverlap`
  (params (OverlappedComponent :type "PrimitiveComponent Object Reference") (OtherActor :type "Actor Object Reference") (OtherComp :type "PrimitiveComponent Object Reference") (OtherBodyIndex :type Integer) (bFromSweep :type Boolean) (SweepResult :type "HitResult Structure (by ref)"))
  ;[1 1 1] Detección de Rango de Ataque (Inicio y Fin del Ataque)
  (bind _asbp_clare_character (cast `/Game/Characters/Clare/Blueprints/BP_ClareCharacter` OtherActor))
  (set `self.CanAttack` true)
  (set `self.PlayerRef` _asbp_clare_character))

(event `self.AttackRange.OnComponentEndOverlap`
  (params (OverlappedComponent :type "PrimitiveComponent Object Reference") (OtherActor :type "Actor Object Reference") (OtherComp :type "PrimitiveComponent Object Reference") (OtherBodyIndex :type Integer))
  ;[1 1 1] Detección de Rango de Ataque (Inicio y Fin del Ataque)
  (cast `/Game/Characters/Clare/Blueprints/BP_ClareCharacter` OtherActor)
  (set `self.CanAttack` false)
  (`self.StarAttackLoop`))

(event `self.ReceiveBeginPlay`
  ;[1 1 1] Inicialización del Enemigo (Velocidad y Barra de Vida)
  (`|ExecutionSequence`
    (:`then_0`
      (set `CharacterMovementComponent.MaxWalkSpeed` (`self.Velocidad`) (`self.CharacterMovement`)))
    (:`then_1`
      (cast `/Game/Characters/Enemies/BP_Rata/WBP_HealthBar` (`WidgetComponent.GetUserWidgetObject` (`self.HealthBarWidget`))))))

(fn `UserConstructionScript`)