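; Francis is an AI customer character that orders at a table and attacks Clare, the player, when patience runs out.
; It walks to the nearest "Table"-tagged actor, then generates a random order and shows its icon.
; A one-second timer drains patience until fury raises walk speed and starts looping chase and range-checked damage timers.
; Debug prints and delays pad most steps, and the delayed-order event OnReachedTable is never called here.
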(event `self.ReceiveBeginPlay`
  (bind _asbp_clare_character (cast `/Game/Characters/Clare/Blueprints/BP_ClareCharacter` (`GameplayStatics.GetPlayerCharacter` 0)))
  ;[1 1 1] Setters for Francis (Inicializando a Francis)
  (set `self.TargetClare` _asbp_clare_character)
  (set `self.Health` (`self.MaxHealth`))
  (set `self.CurrentPatience` (`KismetMathLibrary.RandomFloatInRange` (`self.PatienceMin`) (`self.PatienceMax`)))
  (set `self.OrderPrepTime` (`KismetMathLibrary.RandomFloatInRange` (`self.PatienceForOrderMin`) (`self.PatienceForOrderMax`)))
  (set `self.FrancisState` "NewEnumerator0")
  (set `CharacterMovementComponent.MaxWalkSpeed` (`self.BaseWalkSpeed`) (`self.CharacterMovement`))
  (`self.FindAndMoveToTable`))

(event `FindAndMoveToTable`
  ;[1 1 1] Francis en busqueda de una mesa
  (bind _outactors (`GameplayStatics.GetAllActorsWithTag` "Table"))
  (for _array_element _outactors
    (bind _returnvalue (`KismetMathLibrary.VSize` (- (`self.K2_GetActorLocation` _array_element) (`self.K2_GetActorLocation` self))))
    (if (< _returnvalue (`self.TempNearestDistance`))
      (set `self.TempNearestDistance` _returnvalue)
      (bind _output_get (set `self.TempNearestTable` _array_element))))
  (`/Engine/EditorBlueprintResources/StandardMacros.IsValid` _output_get
    (:`Is Valid`
      (set `self.TargetTable` (`self.TempNearestTable`))
      (`|AIMoveTo` self (0.0 0.0 0.0) (`self.TargetTable`)
        (:`OnSuccess`
          (`KismetSystemLibrary.PrintString` "Se ha encontrado la mesa" true true (struct :`G` 1.0 :`B` 0.048021 :`A` 1.0) 5.0)
          (`KismetSystemLibrary.Delay` 2.0)
          (`self.OnOrderReady`))
        (:`OnFail`
          (`KismetSystemLibrary.Delay` 1.0)
          (`self.FindAndMoveToTable`))))
    (:`Is Not Valid`
      (`KismetSystemLibrary.Delay` 2.0)
      (`self.FindAndMoveToTable`))))

(event `OnReachedTable`
  (set `self.FrancisState` "NewEnumerator5")
  (set `self.HasOrder` false)
  (`KismetSystemLibrary.K2_SetTimerDelegate` (delegate `OnOrderReady`) (`self.OrderPrepTime`)))

(event `OnOrderReady`
  (bind _returnvalue (`KismetMathLibrary.RandomIntegerInRange` 1 10))
  (bind _returnvalue_2 (select `int` (`KismetMathLibrary.RandomIntegerInRange` 0 1) :`0` "NewEnumerator0" :`1` "NewEnumerator1" :!type "/Game/Characters/Francis/Blueprints/E_Texture Enum"))
  (bind _returnvalue_3 (select `int` (`KismetMathLibrary.RandomIntegerInRange` 0 1) :`0` "NewEnumerator0" :`1` "NewEnumerator1" :!type "/Game/Characters/Francis/Blueprints/E_Color Enum"))
  (bind _returnvalue_4 (select `int` (`KismetMathLibrary.RandomIntegerInRange` 0 1) :`0` "NewEnumerator0" :`1` "NewEnumerator1" :!type "/Game/Characters/Francis/Blueprints/E_Flavor Enum"))
  (set `self.HasOrder` true)
  (set `self.OrderData` (make `/Game/Characters/Francis/Blueprints/S_OrderData` _returnvalue _returnvalue_2 _returnvalue_4 _returnvalue_3))
  (set `self.FrancisState` "NewEnumerator7")
  (`SceneComponent.SetVisibility` (`self.W_OrderIcon`) true false)
  (`KismetSystemLibrary.PrintString` (`KismetStringLibrary.Concat_StrStr` "Pedido:" (`KismetStringLibrary.Conv_IntToString` _returnvalue) "--" (`|GetEnumeratorNameAsString` _returnvalue_2) "--" (`|GetEnumeratorNameAsString` _returnvalue_4) "--" (`|GetEnumeratorNameAsString` _returnvalue_3)))
  ;[1 1 1] Debugging para comprobar el llamado del evento
  (`KismetSystemLibrary.PrintString` "OnreachedTable Iniciado" true true (struct :`G` 1.0 :`B` 0.048021 :`A` 1.0) 5.0)
  (`KismetSystemLibrary.Delay` 2.0)
  ;[1 1 1] Cuando Francis alcanza la mesa
  (set `self.FrancisState` "NewEnumerator2")
  (bind _returnvalue_5 (`KismetSystemLibrary.K2_SetTimerDelegate` (delegate `PatienceTick`) 1.0 true)))

(event `EnterFury`
  (`KismetSystemLibrary.PrintString` "EnterFury ejecutado" true true (struct :`G` 1.0 :`B` 0.102467 :`A` 1.0) 5.0)
  (`KismetSystemLibrary.Delay` 2.0)
  (set `self.IsFurious` true)
  (set `self.FrancisState` "NewEnumerator3")
  (set `CharacterMovementComponent.MaxWalkSpeed` (* (`self.BaseWalkSpeed`) (`self.FuriousMultiplier`)) (`self.CharacterMovement`))
  (`self.IsAttacking`))

(event `IsAttacking`
  (`KismetSystemLibrary.PrintString` "IsAttacking ejecutado" true true (struct :`G` 1.0 :`B` 0.102467 :`A` 1.0) 5.0)
  (`KismetSystemLibrary.Delay` 2.0)
  (set `self.FrancisState` "NewEnumerator4")
  (`KismetSystemLibrary.K2_SetTimerDelegate` (delegate `MoveToTargetClare`) 0.25 true)
  (`KismetSystemLibrary.K2_SetTimerDelegate` (delegate `TryAttack`) 1.0 true))

(event `PatienceTick`
  ;[1 1 1] Patience tick (Contador de paciencia despues de ordenar)
  (bind _output_get (set `self.CurrentPatience` (- (`self.CurrentPatience`) 1.0)))
  ;[1 1 1] Debugging para comprobar el timer en gampley
  (`KismetSystemLibrary.DrawDebugString` (0.0 0.0 85.0) (`KismetStringLibrary.Conv_DoubleToString` _output_get) self (struct :`R` 1.0 :`G` 1.0 :`B` 1.0 :`A` 1.0) 1.0)
  (if (<= _output_get 0.0)
    (`KismetSystemLibrary.K2_ClearAndInvalidateTimerHandle` (stale `OnOrderReady` _returnvalue_5))
    ;[1 1 1] Debugging para comprobar el llamado del evento
    (`KismetSystemLibrary.PrintString` "Paciencia agotada, ENTRANDO EN MODO FURIA" true true (struct :`R` 1.0 :`G` 0.016962 :`B` 0.268647 :`A` 1.0) 5.0)
    (`KismetSystemLibrary.Delay` 2.0)
    (`self.EnterFury`)))

(event `TryAttack`
  (`KismetSystemLibrary.PrintString` "TryAttack ejecutado" true true (struct :`G` 1.0 :`B` 0.102467 :`A` 1.0) 5.0)
  (`KismetSystemLibrary.Delay` 2.0)
  (if (<= (`KismetMathLibrary.VSize` (- (`self.K2_GetActorLocation` self) (`self.K2_GetActorLocation` (`self.TargetClare`)))) (`self.AttackRange`))
    (`KismetSystemLibrary.PrintString` "Francis Golpea a Clare" true true (struct :`R` 1.0 :`B` 0.009844 :`A` 1.0))
    (`GameplayStatics.ApplyDamage` (`self.TargetClare`) (`self.AttackDamage`) (`AIBlueprintHelperLibrary.GetAIController` self) self)
    (`KismetSystemLibrary.PrintString` (`KismetStringLibrary.Concat_StrStr` "Daño ejecutado, daño:" (`KismetStringLibrary.Conv_DoubleToString` (`self.AttackDamage`))))))

(event `MoveToTargetClare`
  ;[1 1 1] Francis moviendose a Clare
  (`KismetSystemLibrary.PrintString` "MOVETOTARGET ejecutado" true true (struct :`G` 1.0 :`B` 0.102467 :`A` 1.0) 5.0)
  (`KismetSystemLibrary.Delay` 2.0)
  (`self.TargetClare`
    (:`then`
      (if true
        (if (`|EnumEquality` (`self.FrancisState`) "NewEnumerator4")
          (`|AIMoveTo` self (0.0 0.0 0.0) (`self.TargetClare`) (`self.Acceptance Radius`))
          (else
            (`KismetSystemLibrary.PrintString` "ERROR!" true true (struct :`R` 1.0 :`B` 0.005894 :`A` 1.0))))
        (else
          (`KismetSystemLibrary.PrintString` "ERROR!" true true (struct :`R` 1.0 :`B` 0.005894 :`A` 1.0)))))
    (:`else`)))

(fn `UserConstructionScript`)