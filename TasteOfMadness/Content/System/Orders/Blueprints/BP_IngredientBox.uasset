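; BP_IngredientBox is an ingredient crate that spawns the ingredient actors of the store selected in the order manager.
; AbrirCaja runs on BeginPlay, finds BP_OrderManager, clears TiendaSeleccionada, then reads its ingredient list, mapping each entry to a Blueprint class spawned at SpawnPoint.
; BoxCollision overlaps with BP_ClareCharacter print range prompts, but both set JugadorEnRango false, so the input action that reopens the box never passes its check.
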(event `self.ReceiveBeginPlay`
  (`self.AbrirCaja`))

(event `self.BoxCollision.OnComponentBeginOverlap`
  (params (OverlappedComponent :type "PrimitiveComponent Object Reference") (OtherActor :type "Actor Object Reference") (OtherComp :type "PrimitiveComponent Object Reference") (OtherBodyIndex :type Integer) (bFromSweep :type Boolean) (SweepResult :type "HitResult Structure (by ref)"))
  ;[1 1 1] Comment
  (cast `/Game/Characters/Clare/Blueprints/BP_ClareCharacter` OtherActor)
  (set `self.JugadorEnRango` false)
  (`KismetSystemLibrary.PrintString` "\"Presiona T para abrir\""))

(event `self.BoxCollision.OnComponentEndOverlap`
  (params (OverlappedComponent :type "PrimitiveComponent Object Reference") (OtherActor :type "Actor Object Reference") (OtherComp :type "PrimitiveComponent Object Reference") (OtherBodyIndex :type Integer))
  ;[1 1 1] Comment
  (cast `/Game/Characters/Clare/Blueprints/BP_ClareCharacter` OtherActor)
  (set `self.JugadorEnRango` false)
  (`KismetSystemLibrary.PrintString` "\"Fuera de rango\""))

(event `InputAction|AbrirCaja`
  (params (Key :type "Key Structure"))
  (:`Pressed`
    (if (`self.JugadorEnRango`)
      (`self.AbrirCaja`))))

(fn `AbrirCaja`
  (bind _outactors (`GameplayStatics.GetAllActorsOfClass` "/Game/System/Orders/Blueprints/BP_OrderManager.BP_OrderManager_C"))
  (set `self.OrderManagerRef` (`|GetArrayItem` _outactors))
  (bind _output_get (set `/Game/System/Orders/Blueprints/BP_OrderManager.TiendaSeleccionada` (struct) (`self.OrderManagerRef`)))
  (bind (_nombretienda _costoentrega _tiempoentrega _estaabierta _ingredientes _cantidadingredientes) (break `/Game/System/Orders/Data/ST_StoreInfo` _output_get))
  (for _index (range _cantidadingredientes)
    (switch `string` (`|GetArrayItem` _ingredientes _index)
      (:`S_Butter`
        (set `self.ClaseIngrediente` "/Game/System/Orders/Comida/BP_Butter.BP_Butter_C"))
      (:`S_Chesse`
        (set `self.ClaseIngrediente` "/Game/System/Orders/Comida/BP_Chesse.BP_Chesse_C"))
      (:`S_Corn`
        (set `self.ClaseIngrediente` "/Game/System/Orders/Comida/BP_Corn.BP_Corn_C"))
      (:`S_Cream`
        (set `self.ClaseIngrediente` "/Game/System/Orders/Comida/BP_Cream.BP_Cream_C"))
      (:`S_Eggs`
        (set `self.ClaseIngrediente` "/Game/System/Orders/Comida/BP_Eggs.BP_Eggs_C"))
      (:`S_Garlic`
        (set `self.ClaseIngrediente` "/Game/System/Orders/Comida/BP_Garlic.BP_Garlic_C"))
      (:`S_Milk`
        (set `self.ClaseIngrediente` "/Game/System/Orders/Comida/BP_Milk.BP_Milk_C"))
      (:`S_Noodles`
        (set `self.ClaseIngrediente` "/Game/System/Orders/Comida/BP_Noodles.BP_Noodles_C"))
      (:`S_Potato`
        (set `self.ClaseIngrediente` "/Game/System/Orders/Comida/BP_Potato.BP_Potato_C"))
      (:`S_Squash`
        (set `self.ClaseIngrediente` "/Game/System/Orders/Comida/BP_Squash.BP_Squash_C")))
    (`|SpawnActorFromClass` (`self.ClaseIngrediente`) (`SceneComponent.K2_GetComponentToWorld` (`self.SpawnPoint`)) "Undefined" "OverrideRootScale" null null)))

(fn `UserConstructionScript`)