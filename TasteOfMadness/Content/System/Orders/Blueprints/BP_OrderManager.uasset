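; Order manager actor that holds the game's ingredient stores and tracks a single active delivery order.
; On BeginPlay it fills TiendasInfo with five hardcoded stores and lists all available ingredients.
; Each store randomizes its open state, cost, delivery time and ingredient count within tiers, where pricier stores generally deliver faster and carry more.
; IniciarPedido copies TiendaSeleccionada into PedidoActual unless an order is running; it never checks open state or completes orders.
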(event `self.ReceiveBeginPlay`
  ;[1 1 1] Inicio del sistema de pedidos
  (`self.InicializarTiendas`)
  (set `self.IngredientesDisponibles` (`|MakeArray` "S_Butter" "S_Cheese" "S_Corn" "S_Cream" "S_Eggs" "S_Garlic" "S_Milk" "S_Noodles" "S_Potato" "S_Squash")))

(event `InicializarTiendas`
  ;[1 1 1] Carga inicial de las tiendas
  (`KismetArrayLibrary.Array_Add` (`self.TiendasInfo`) (make `/Game/System/Orders/Data/ST_StoreInfo` "Super Terraverde" (`KismetMathLibrary.RandomFloatInRange` 10.0 20.0) (`KismetMathLibrary.RandomFloatInRange` 40.0 60.0) (`KismetMathLibrary.RandomBool`) (`|MakeArray` "S_Corn" "S_Potato" "S_Squash" "S_Cheese") (`KismetMathLibrary.RandomIntegerInRange` 2 5)))
  (`KismetArrayLibrary.Array_Add` (`self.TiendasInfo`) (make `/Game/System/Orders/Data/ST_StoreInfo` "Abarrotes Eridoria" (`KismetMathLibrary.RandomFloatInRange` 20.0 30.0) (`KismetMathLibrary.RandomFloatInRange` 40.0 50.0) (`KismetMathLibrary.RandomBool`) (`|MakeArray` "S_Potato" "S_Milk" "S_Butter" "S_Eggs" "S_Cheese") (`KismetMathLibrary.RandomIntegerInRange` 4 7)))
  (`KismetArrayLibrary.Array_Add` (`self.TiendasInfo`) (make `/Game/System/Orders/Data/ST_StoreInfo` "AquaShop" (`KismetMathLibrary.RandomFloatInRange` 30.0 50.0) (`KismetMathLibrary.RandomFloatInRange` 30.0 40.0) (`KismetMathLibrary.RandomBool`) (`|MakeArray` "S_Milk" "S_Cream" "S_Eggs" "S_Squash" "S_Noodles" "S_Butter") (`KismetMathLibrary.RandomIntegerInRange` 7 10)))
  (`KismetArrayLibrary.Array_Add` (`self.TiendasInfo`) (make `/Game/System/Orders/Data/ST_StoreInfo` "UltraMarket Ignis" (`KismetMathLibrary.RandomFloatInRange` 50.0 70.0) (`KismetMathLibrary.RandomFloatInRange` 20.0 30.0) (`KismetMathLibrary.RandomBool`) (`|MakeArray` "S_Cheese" "S_Cream" "S_Noodles" "S_Garlic" "S_Eggs" "S_Butter") (`KismetMathLibrary.RandomIntegerInRange` 9 12)))
  (`KismetArrayLibrary.Array_Add` (`self.TiendasInfo`) (make `/Game/System/Orders/Data/ST_StoreInfo` "Comida Clara" (`KismetMathLibrary.RandomFloatInRange` 70.0 100.0) (`KismetMathLibrary.RandomFloatInRange` 10.0 20.0) (`KismetMathLibrary.RandomBool`) (`|MakeArray` "S_Butter" "S_Cheese" "S_Corn" "S_Cream" "S_Eggs" "S_Garlic" "S_Milk" "S_Noodles" "S_Potato" "S_Squash") (`KismetMathLibrary.RandomIntegerInRange` 12 15))))

(fn `IniciarPedido`
  (if (`self.PedidoEnProgreso`)
    (`KismetSystemLibrary.PrintString` "“Ya hay un pedido en curso”")
    (else
      (set `self.PedidoEnProgreso` true)
      (set `self.PedidoActual` (`self.TiendaSeleccionada`)))))

(fn `UserConstructionScript`)