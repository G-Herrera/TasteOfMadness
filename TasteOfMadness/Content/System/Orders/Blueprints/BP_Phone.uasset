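; BP_Phone is an interactable phone actor that opens the shop menu, linked to the order system.
; Its trigger shows an F prompt and enables input while BP_ClareCharacter overlaps, reversing both on exit.
; Pressing F creates WBP_TiendaMenu with the first BP_OrderManager found and switches to UI-only input with cursor.
; TiendaMenuRef guards creation but is never assigned here, and JugadorEnRango is only ever set false.
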(event `Key|F`
  (params (Key :type "Key Structure"))
  (bind _returnvalue (`GameplayStatics.GetPlayerController` 0))
  (:`Pressed`
    (if true
      (bind _outactors (`GameplayStatics.GetAllActorsOfClass` "/Game/System/Orders/Blueprints/BP_OrderManager.BP_OrderManager_C"))
      (if (not (`KismetSystemLibrary.IsValid` (`self.TiendaMenuRef`)))
        (bind _returnvalue_2 (`|CreateWidget` "/Game/System/Orders/Widgets/WBP_TiendaMenu.WBP_TiendaMenu_C" null (`|GetArrayItem` _outactors)))
        (`UserWidget.AddToViewport` _returnvalue_2 0)
        (set `PlayerController.bShowMouseCursor` true _returnvalue)
        (`WidgetBlueprintLibrary.SetInputMode_UIOnlyEx` _returnvalue null)))))

(event `self.InteractionTrigger.OnComponentBeginOverlap`
  (params (OverlappedComponent :type "PrimitiveComponent Object Reference") (OtherActor :type "Actor Object Reference") (OtherComp :type "PrimitiveComponent Object Reference") (OtherBodyIndex :type Integer) (bFromSweep :type Boolean) (SweepResult :type "HitResult Structure (by ref)"))
  ;[1 1 1] Interaccion con el telefono
  (cast `/Game/Characters/Clare/Blueprints/BP_ClareCharacter` OtherActor)
  (set `self.JugadorEnRango` false)
  (`SceneComponent.SetVisibility` (`self.WidgetInteraccionF`) true false)
  (`self.EnableInput` (`GameplayStatics.GetPlayerController` 0)))

(event `self.InteractionTrigger.OnComponentEndOverlap`
  (params (OverlappedComponent :type "PrimitiveComponent Object Reference") (OtherActor :type "Actor Object Reference") (OtherComp :type "PrimitiveComponent Object Reference") (OtherBodyIndex :type Integer))
  ;[1 1 1] Interaccion con el telefono
  (cast `/Game/Characters/Clare/Blueprints/BP_ClareCharacter` OtherActor)
  (set `self.JugadorEnRango` false)
  (`SceneComponent.SetVisibility` (`self.WidgetInteraccionF`) false false)
  (`self.DisableInput` (`GameplayStatics.GetPlayerController` 0)))

(fn `UserConstructionScript`)